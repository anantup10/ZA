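; Shotgun weapon Blueprint that fires a spread of hitscan pellets from the player camera.
; WeaponTrace loops thin sphere traces in random directions within a cone, with debug drawing on.
; Hit actors implementing BPI_Damage receive a damage message carrying Points.
; Points then increments if HitRelevence is true, otherwise resets to one; the flag is cleared before tracing and never set true in this graph.
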(event `self.Weapon Trace`
  (bind _transformcomponent (`PlayerCameraManager.TransformComponent` (`GameplayStatics.GetPlayerCameraManager` 0)))
  (bind _returnvalue (`SceneComponent.K2_GetComponentLocation` _transformcomponent))
  (set `self.HitRelevence` false)
  (for _ (range 9)
    (bind _outhit (`KismetSystemLibrary.SphereTraceSingle` :`Start` _returnvalue :`End` (+ (* 8000.0 (`KismetMathLibrary.RandomUnitVectorInConeInDegrees` (`SceneComponent.GetForwardVector` _transformcomponent) (`self.Cone Half Angle in Degrees`))) _returnvalue) :`Radius` 1.0 :`TraceChannel` "TraceTypeQuery1" :`DrawDebugType` "ForDuration"))
    (bind (_bblockinghit _binitialoverlap _time _distance _location _impactpoint _normal _impactnormal _physmat _hitactor) (`GameplayStatics.BreakHitResult` _outhit))
    (if (`KismetSystemLibrary.DoesImplementInterface` _hitactor "/Game/Blueprints/Weapons/BPI_Damage.BPI_Damage_C")
      (message `/Game/Blueprints/Weapons/BPI_Damage.RecieveDamage` _hitactor (`self.Points`))))
  (if (`self.HitRelevence`)
    (`/Engine/EditorBlueprintResources/StandardMacros.IncrementInt` (`self.Points`))
    (else
      (set `self.Points` 1))))

(fn `UserConstructionScript`
  (`parent.UserConstructionScript`))