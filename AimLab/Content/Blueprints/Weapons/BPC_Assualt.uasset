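; Assault weapon Blueprint that fires a hitscan trace and scales its damage message with consecutive hits.
; WeaponTrace takes the impact point of a camera trace, then sphere-traces from the Arrow toward it so shots originate at the weapon yet follow the aim.
; Actors implementing BPI_Damage receive an incrementing Points value through RecieveDamageMessage; any other trace result resets Points to zero.
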(event `self.Weapon Trace`
  (bind _points (`self.Points`))
  (bind _returnvalue (`SceneComponent.K2_GetComponentLocation` (`self.Arrow`)))
  (bind _outhit (`/Game/Blueprints/Liberaries/BPFL.CameraTrace` 8000.0 2.0))
  (bind _outhit_2 (`KismetSystemLibrary.SphereTraceSingle` _returnvalue (+ (* (`KismetMathLibrary.GetForwardVector` (`KismetMathLibrary.FindLookAtRotation` _returnvalue (`.ImpactPoint` (`GameplayStatics.BreakHitResult` _outhit)))) 8000.0) _returnvalue) 1.0 "TraceTypeQuery1"))
  (bind (_bblockinghit _binitialoverlap _time _distance _location _impactpoint _normal _impactnormal _physmat _hitactor) (`GameplayStatics.BreakHitResult` _outhit_2))
  (if (`KismetSystemLibrary.DoesImplementInterface` _hitactor "/Game/Blueprints/Weapons/BPI_Damage.BPI_Damage_C")
    (set `self.Points` (+ _points 1))
    (message `/Game/Blueprints/Weapons/BPI_Damage.RecieveDamage` _hitactor _points)
    (else
      (set `self.Points` 0))))

(fn `UserConstructionScript`
  (`parent.UserConstructionScript`))