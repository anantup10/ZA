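; Base weapon Blueprint that handles firing, magazine ammo, reloading and exposes an FOV multiplier.
; Firing spends a round, spawns muzzle particles and sound at the Arrow component, then calls WeaponTrace, an empty event here.
; An empty magazine triggers an automatic reload, also callable through Reload.
; Reloading shows a WB_reload widget animation and refills ammo after ReloadTime, with no guard against firing or re-triggering meanwhile.
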(event `self.ReceiveBeginPlay`
  (set `self.Ammo` (`self.MaxMagazineAmmo`)))

(event `/Game/Blueprints/FirstPersonTemplate/BPI_weapon.FireWeapon`
  (`/Engine/EditorBlueprintResources/StandardMacros.CompareInt` (`self.Ammo`) :!label _label
    (:`>`
      (set `self.Ammo` (- (`self.Ammo`) 1))
      (`self.WeaponFireEffects`)
      (`self.Weapon Trace`)
      (`/Engine/EditorBlueprintResources/StandardMacros.CompareInt` (`self.Ammo`)
        (:`==`
          _)
        (:`<`
          _))
      (`self.ReloadWeapon`))
    (:`==`
      (`self.ReloadWeapon` :!label _label_2))
    (:`<`
      (goto _label_2))))

(event `Weapon Trace`)

(event `WeaponFire`
  (goto _label))

(event `ReloadWeapon`
  (bind _returnvalue (`|CreateWidget` "/Game/Blueprints/Weapons/WB_reload.WB_reload_C" :!label _label_3))
  (`/Game/Blueprints/Weapons/WB_reload.Reload Animation` _returnvalue (`self.ReloadTime`))
  (`UserWidget.AddToViewport` _returnvalue 0)
  (`KismetSystemLibrary.Delay` (`self.ReloadTime`))
  (set `self.Ammo` (`self.MaxMagazineAmmo`)))

(event `/Game/Blueprints/FirstPersonTemplate/BPI_weapon.Reload`
  (goto _label_3))

(fn `FOVmultiplier`
  (returns (FOVmul :type "Float (double-precision)"))
  (return (`self.FOVmul`)))

(fn `UserConstructionScript`)

(fn `WeaponFireEffects`
  (bind (_returnvalue_location _returnvalue_rotation) (`KismetMathLibrary.BreakTransform` (`SceneComponent.K2_GetComponentToWorld` (`self.Arrow`))))
  (`GameplayStatics.SpawnEmitterAtLocation` (`self.Weapon Fire Emitter`) _returnvalue_location _returnvalue_rotation (`self.WeaponFireScale`))
  (`GameplayStatics.SpawnSoundAtLocation` (`self.WeaponFIreSound`) _returnvalue_location (struct) 1.0 1.0 0.0 null null))